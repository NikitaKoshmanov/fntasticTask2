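; BP_Button2 is an interactable push button that fires CallDispatcher2 and plays a sound when pressed.
; A box overlap with the DefaultPawn opens and closes a gate, so the Interact2 input only works while the player is nearby.
; On press, two timelines lerp the button mesh into a recessed position and back, using transforms cached at BeginPlay.
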(event OnComponentBeginOverlap(Box2)
  (params (OverlappedComponent :type Primitive%20Component%20Object%20Reference) (OtherActor :type Actor%20Object%20Reference) (OtherComp :type Primitive%20Component%20Object%20Reference) (OtherBodyIndex :type Integer) (bFromSweep :type Boolean) (SweepResult :type Hit%20Result%20Structure%20%28by%20ref%29))
  (Utilities|Casting|CastToDefaultPawn OtherActor)
  (Utilities|FlowControl|Gate true) ; enters at Open
)

(event OnComponentEndOverlap(Box2)
  (params (OverlappedComponent :type Primitive%20Component%20Object%20Reference) (OtherActor :type Actor%20Object%20Reference) (OtherComp :type Primitive%20Component%20Object%20Reference) (OtherBodyIndex :type Integer))
  (Utilities|Casting|CastToDefaultPawn OtherActor)
  (Utilities|FlowControl|Gate true) ; enters at Close
)

(event EventBeginPlay
  (bind _button2 (Variables|Default|GetButton2))
  (bind _returnvalue (Transformation|GetRelativeTransform _button2))
  (Variables|Default|SetOut%20Position (Math|Transform|MakeTransform (.location _returnvalue) (.rotation _returnvalue) (.scale _returnvalue)))
  (Variables|Default|SetIn%20Position (Math|Transform|MakeTransform (- (.location _returnvalue) "0, 0,30.000000") (.rotation _returnvalue) (.scale _returnvalue)))
  (Input|EnableInput (Game|GetPlayerController 0)))

(event Input|ActionEvents|InputActionInteract2
  (params (Key :type Key%20Structure :default "None"))
  (:Pressed
    (Utilities|FlowControl|Gate true
      (:Exit
        (Default|CallDispatcher2)
        (Audio|PlaySoundatLocation "/Game/Assets/button.button" (Transformation|GetActorLocation) "0, 0, 0" 1.0 1.0 0.0 0 0 0)
        (bind _button_in (Timeline|Timeline_0 PlayFromStart)
          (:Update
            (Transformation|SetRelativeTransform (Variables|Default|GetButton2) (Math|Transform|Lerp(Transform) (Variables|Default|GetOut%20Position) (Variables|Default|GetIn%20Position) _button_in) false false))
          (:Finished
            (bind _button_in_2 (Timeline|Timeline_1 ReverseFromEnd)
              (:Update
                (Transformation|SetRelativeTransform (Variables|Default|GetButton2) (Math|Transform|Lerp(Transform) (Variables|Default|GetOut%20Position) (Variables|Default|GetIn%20Position) _button_in_2) false false)))))))))

(fn ConstructionScript)