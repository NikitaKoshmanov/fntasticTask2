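; BP_Button is an interactable push button that fires an event dispatcher when pressed.
; Box overlaps by a DefaultPawn open and close a gate, which lets the Interact input through only while open.
; A press calls the dispatcher, then plays a sound and chained timelines that lerp the button 30 units down and back between transforms cached at BeginPlay.
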(event OnComponentBeginOverlap(Box)
  (params (OverlappedComponent :type Primitive%20Component%20Object%20Reference) (OtherActor :type Actor%20Object%20Reference) (OtherComp :type Primitive%20Component%20Object%20Reference) (OtherBodyIndex :type Integer) (bFromSweep :type Boolean) (SweepResult :type Hit%20Result%20Structure%20%28by%20ref%29))
  ;[1 1 1] Push Button
  (Utilities|Casting|CastToDefaultPawn OtherActor)
  (Variables|Default|SetIn%20Trigger true)
  (Utilities|FlowControl|Gate true) ; enters at Open
)

(event OnComponentEndOverlap(Box)
  (params (OverlappedComponent :type Primitive%20Component%20Object%20Reference) (OtherActor :type Actor%20Object%20Reference) (OtherComp :type Primitive%20Component%20Object%20Reference) (OtherBodyIndex :type Integer))
  ;[1 1 1] Push Button
  (Utilities|Casting|CastToDefaultPawn OtherActor)
  (Variables|Default|SetIn%20Trigger false)
  (Utilities|FlowControl|Gate true) ; enters at Close
)

(event EventBeginPlay
  (bind _button (Variables|Default|GetButton))
  (bind _returnvalue (Transformation|GetRelativeTransform _button))
  (Variables|Default|SetOut%20Position (Math|Transform|MakeTransform (.location _returnvalue) (.rotation _returnvalue) (.scale _returnvalue)))
  (Variables|Default|SetIn%20Position (Math|Transform|MakeTransform (- (.location _returnvalue) "0, 0,30.000000") (.rotation _returnvalue) (.scale _returnvalue)))
  (Input|EnableInput (Game|GetPlayerController 0)))

(event Input|ActionEvents|InputActionInteract
  (params (Key :type Key%20Structure :default "None"))
  ;[1 1 1] Push Button
  (:Pressed
    (Utilities|FlowControl|Gate true
      (:Exit
        (Default|CallDispatcher)
        (|ButtonAnimation)))))

(fn ConstructionScript)